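; BP_WeaponWorld is a world-placed weapon actor whose type is chosen by its Weapon row name.
; Its construction script looks that row up in the DT_Weapons data table and, if found, copies damage, force, range, mesh and sound effects into its variables.
; It then applies the mesh to the WeaponModel component, so the model updates in the editor.
; The event graph has no active logic.
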(event EventBeginPlay)

(event Collision|EventActorBeginOverlap
  (params (OtherActor :type Actor%20Object%20Reference)))

(event EventTick
  (params (DeltaSeconds :type Float%20%28single-precision%29)))

(fn ConstructionScript
  (bind _weapon (Variables|Default|GetWeapon))
  (bind _returnvalue (Class|DataTableFunctionLibrary|DoesDataTableRowExist "/Game/FirstPerson/Blueprints/Weapon/DT_Weapons.DT_Weapons" _weapon))
  (if _returnvalue
    (bind _returnvalue_2 (Utilities|GetDataTableRow "/Game/FirstPerson/Blueprints/Weapon/DT_Weapons.DT_Weapons" _weapon)
      (:then
        (Variables|Default|SetDamage (.damage _returnvalue_2))
        (Variables|Default|SetForce (.force _returnvalue_2))
        (Variables|Default|SetRange (.range _returnvalue_2))
        (Variables|Default|SetModel (.model _returnvalue_2))
        (Variables|Default|SetShootSFX (.shootsfx _returnvalue_2))
        (Variables|Default|SetReloadSFX (.reloadsfx _returnvalue_2))
        (Variables|Default|SetDryFireSFX (.dryfiresfx _returnvalue_2))
        (Components|StaticMesh|SetStaticMesh (Variables|Default|GetWeaponModel) (Variables|Default|GetModel))))))