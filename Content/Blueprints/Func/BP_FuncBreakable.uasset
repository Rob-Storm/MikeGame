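; BP_FuncBreakable is a breakable prop that loses health when shot and shatters at zero.
; Shots route through server-to-multicast RPCs, so each machine decrements Health itself and plays hit sounds.
; Breaking hides the cube, disables its collision and plays an effect and sound, without destroying the actor.
; The construction script picks effect and sounds from MaterialType, with only Glass defined.
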(event Custom|RPCMulticast_Destroy
  (bind _cube (Variables|Default|GetCube))
  (Niagara|SpawnSystematLocation (Variables|Default|GetDestructionEffect) (Transformation|GetActorLocation))
  (Collision|SetCollisionEnabled _cube "NoCollision")
  (Rendering|SetVisibility _cube false false)
  (Audio|PlaySoundatLocation (Variables|Default|GetBreakSound) (Transformation|GetActorLocation) "0, 0, 0" 1.0 1.0 0.0 0 0 0 0))

(event Custom|RPCServer_Destroy
  (CallFunction|RPCMulticastDestroy))

(event Custom|RPCServer_Damage
  (params (Damage :type Float%20%28double-precision%29) (Location :type Vector))
  (CallFunction|RPCMulticastDamage Damage Location))

(event Custom|RPCMulticast_Damage
  (params (Damage :type Float%20%28double-precision%29) (Location :type Vector))
  (bind _output_get (Variables|Default|SetHealth (- (Variables|Default|GetHealth) Damage)))
  (if (<= _output_get 0.0)
    (CallFunction|RPCServerDestroy)
    (else
      (CallFunction|RPCMulitcastPlaySound (Variables|Default|GetHitSound) Location))))

(event Custom|RPCMulitcast_PlaySound
  (params (Sound :type Sound%20Base%20Object%20Reference) (Location :type Vector))
  (Audio|PlaySoundatLocation Sound Location "0, 0, 0" 1.0 1.0 0.0 0 0 0 0))

(event EventShot
  (params (Damage :type Float%20%28double-precision%29) (Location :type Vector :default "0, 0, 0"))
  (CallFunction|RPCServerDamage Damage Location))

(fn ConstructionScript
  (switch Utilities|FlowControl|Switch|SwitchonEN_MaterialType (Variables|Default|GetMaterialType)
    (:NewEnumerator0
      (Variables|Default|SetDestructionEffect "/Game/ParticleEffects/NS_GlassShatter.NS_GlassShatter")
      (Variables|Default|SetHitSound "/Game/Sounds/Glass/SC_GlassBulletHit.SC_GlassBulletHit")
      (Variables|Default|SetBreakSound "/Game/Sounds/Glass/SC_GlassDestroy.SC_GlassDestroy"))))