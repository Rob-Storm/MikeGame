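; BP_FuncElevator is an elevator actor that travels between preset ElevatorLocations when triggered by a non-player Interact call.
; The Interact flag selects the destination index for MoveElevator, which restarts a timeline that sets actor location without sweep.
; Each update lerps from the current location rather than a cached start, so motion compounds toward the target.
; BeginPlay converts Speed, divided by 100, into the timeline play rate.
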(event Custom|MoveElevator
  (params (Level :type Integer))
  (bind _alpha (Timeline|TL_Interp PlayFromStart)
    (:Update
      (Transformation|SetActorLocation (Math|Vector|Lerp(Vector) (Transformation|GetActorLocation) (Utilities|Array|Get(acopy) (Variables|Default|GetElevatorLocations) Level) _alpha) false false))))

(event EventBeginPlay
  (Variables|Default|SetSpeed (/ (Variables|Default|GetSpeed) 1e+02))
  (Components|Timeline|SetPlayRate (Variables|Default|GetTL_Interp) (Variables|Default|GetSpeed)))

(event EventInteract
  (params (Called%20By%20Player? :type Boolean) (Flag :type Integer) (PlayerCaller :type BP%20First%20Person%20Character%20Object%20Reference))
  (if (not Called%20By%20Player?)
    (CallFunction|MoveElevator Flag)))

(fn ConstructionScript)