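; BP_Door is an interactable, lockable door that swings between open and closed.
; Interact plays the locked sound when Locked is set, otherwise it plays the open sound and calls ToggleDoor.
; ToggleDoor flips the Open flag and snaps the Hinge to a stored world rotation, without interpolation.
; Sounds play at the actor's location through an event named as a client RPC.
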(event Custom|RPCClient_FX
  (params (Sound :type Sound%20Wave%20Object%20Reference))
  (Audio|PlaySoundatLocation Sound (Transformation|GetActorLocation) "0, 0, 0" 0.5 1.0 0.0 0 0 0 0))

(event Custom|ToggleDoor
  (bind _hinge (Variables|Default|GetHinge))
  (if (Variables|Default|GetOpen?)
    (Variables|Default|SetOpen? false)
    (Transformation|SetWorldRotation _hinge (Variables|Default|GetCloseRotation) false false)
    (else
      (Variables|Default|SetOpen? true)
      (Transformation|SetWorldRotation _hinge (Variables|Default|GetOpenRotation) false false))))

(event EventInteract
  (if (Variables|Default|GetLocked?)
    (CallFunction|RPCClientFX (Variables|Default|GetLockedSound))
    (else
      (CallFunction|RPCClientFX (Variables|Default|GetOpenSound))
      (CallFunction|ToggleDoor))))

(fn ConstructionScript)