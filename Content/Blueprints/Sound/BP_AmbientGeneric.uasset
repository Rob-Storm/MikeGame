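; BP_AmbientGeneric is a networked sound emitter that plays a configurable sound at its own location.
; It triggers on BeginPlay when PlayOnAwake is set, or whenever Interact is called, acting only with authority in both cases.
; A server RPC forwards to a multicast RPC, which plays the sound with the configured volume, pitch and start time.
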(event Custom|RPCMulticast_PlaySound
  (Audio|PlaySoundatLocation (Variables|Default|GetSoundWave) (Transformation|GetActorLocation) "0, 0, 0" (Variables|Default|GetVolume) (Variables|Default|GetPitch%20Multiplier) (Variables|Default|GetStart%20Time) 0 0 0 0))

(event Custom|RPCServer_PlaySound
  (CallFunction|RPCMulticastPlaySound))

(event EventBeginPlay
  (if (Variables|Default|GetPlayOnAwake?)
    (Networking|SwitchHasAuthority
      (:Authority
        (CallFunction|RPCServerPlaySound)))))

(event EventInteract
  (Networking|SwitchHasAuthority
    (:Authority
      (CallFunction|RPCServerPlaySound))))

(fn ConstructionScript)