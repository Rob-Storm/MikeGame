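; BP_WeaponBase is a base weapon actor that players pick up by interacting with it.
; Interact calls a server RPC that multicasts the pickup, adding the weapon to the caller's BPWeaponInventory, hiding it, disabling model collision and playing a sound.
; ForwardTrace only computes start point, end point and force vector from a camera, without tracing.
; The construction script's weapon-table lookup for stats, mesh and sounds is disconnected.
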(event Custom|RPCMulticast_Pickup
  (params (PlayerCaller :type BP%20First%20Person%20Character%20Object%20Reference))
  (Default|AddWeapon (Variables|/Game/FirstPerson/Blueprints/BP_FirstPersonCharacter.BP_FirstPersonCharacter_C|GetBP_WeaponInventory PlayerCaller) self)
  (Rendering|SetVisibility (Variables|Default|GetDefaultSceneRoot) false true)
  (Collision|SetCollisionEnabled (Variables|Default|GetWeaponModel) "NoCollision")
  (Audio|PlaySoundatLocation "/Game/Sounds/Weapon/itempickup.itempickup" (Transformation|GetActorLocation) "0, 0, 0" 1.0 1.0 0.0 0 0 0 0))

(event Custom|RPCServer_Pickup
  (params (PlayerCaller :type BP%20First%20Person%20Character%20Object%20Reference))
  (CallFunction|RPCMulticastPickup PlayerCaller))

(event EventBeginPlay)

(event EventInteract
  (params (Called%20By%20Player? :type Boolean) (Flag :type Integer) (PlayerCaller :type BP%20First%20Person%20Character%20Object%20Reference))
  (CallFunction|RPCServerPickup PlayerCaller))

(fn ConstructionScript)

(fn ForwardTrace
  (params (Camera :type Scene%20Component%20Object%20Reference) (Range :type Float%20%28double-precision%29) (Force :type Float%20%28double-precision%29))
  (bind _returnvalue (Transformation|GetWorldRotation Camera))
  (bind _returnvalue_2 (Transformation|GetWorldLocation Camera))
  (bind _returnvalue_3 (Math|Vector|GetForwardVector _returnvalue))
  (return _returnvalue_2 (+ _returnvalue_2 (* _returnvalue_3 Range)) (* _returnvalue_3 Force)))