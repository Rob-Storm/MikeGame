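; BP_Button is an interactable, lockable button that triggers a list of affected actors when used.
; Interact runs only with authority, calling a server event that checks Locked and multicasts either the use or locked sound, unless Silent.
; When unlocked, a second multicast sends InteractMessage to every affected actor implementing BPI_Interaction, so their reactions run on server and clients.
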(event Custom|RPCMulticast_ButtonUse
  (for _array_element (Variables|Default|GetAffected%20Actors)
    (if (Utilities|DoesObjectImplementInterface _array_element "/Game/FirstPerson/Blueprints/BPI_Interaction.BPI_Interaction_C")
      (Class|BPIInteraction|Interact(Message) _array_element false))))

(event Custom|RPCServer_ButtonUse
  (if (not (Variables|Default|GetLocked?))
    (CallFunction|RPCMulticastFX (Variables|Default|GetUseSound))
    (CallFunction|RPCMulticastButtonUse)
    (else
      (CallFunction|RPCMulticastFX (Variables|Default|GetLockedSound)))))

(event Custom|RPCMulticast_FX
  (params (Sound :type Sound%20Wave%20Object%20Reference))
  (if (not (Variables|Default|GetSilent?))
    (Audio|PlaySoundatLocation Sound (Transformation|GetActorLocation) "0, 0, 0" 0.5 1.0 0.0 0 0 0 0)))

(event EventInteract
  (params (Called%20By%20Player? :type Boolean))
  (Networking|SwitchHasAuthority
    (:Authority
      (CallFunction|RPCServerButtonUse))))

(fn ConstructionScript)