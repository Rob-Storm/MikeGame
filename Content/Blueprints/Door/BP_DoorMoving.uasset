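; BP_DoorMoving is an interactable, lockable door that snaps between its starting position and an offset one.
; Interact can refuse player-initiated use, plays a locked sound when locked, and otherwise plays the open sound and toggles the Open state.
; Open's RepNotify replays the sound and teleports the actor by OpenOffset or back to the location saved at BeginPlay, which also seeds Open as the inverse of StartOpen.
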(event Custom|RPCClient_FX
  (params (Sound :type Sound%20Wave%20Object%20Reference))
  (Audio|PlaySoundatLocation Sound (Transformation|GetActorLocation) "0, 0, 0" 0.5 1.0 0.0 0 0 0 0))

(event Custom|ToggleDoor
  (if (Variables|Default|GetOpen?)
    (Variables|Default|SetOpen? false)
    (else
      (Variables|Default|SetOpen? true))))

(event EventBeginPlay
  (Variables|Default|SetOpenLocation (Transformation|GetActorLocation))
  (Variables|Default|SetOpen? (not (Variables|Default|GetStartOpen?))))

(event EventInteract
  (params (Called%20By%20Player? :type Boolean) (Flag :type Integer) (PlayerCaller :type BP%20First%20Person%20Character%20Object%20Reference))
  (if (not (and Called%20By%20Player? (Variables|Default|GetPlayerNOTOpen)))
    (if (Variables|Default|GetLocked?)
      (CallFunction|RPCClientFX (Variables|Default|GetLockedSound))
      (else
        (CallFunction|RPCClientFX (Variables|Default|GetOpenSound))
        (CallFunction|ToggleDoor)))))

(fn ConstructionScript)

(fn OnRepOpen?
  (CallFunction|RPCClientFX (Variables|Default|GetOpenSound))
  (if (Variables|Default|GetOpen?)
    (Transformation|AddActorWorldOffset (Variables|Default|GetOpenOffset) false true)
    (else
      (Transformation|SetActorLocation (Variables|Default|GetOpenLocation) false true))))