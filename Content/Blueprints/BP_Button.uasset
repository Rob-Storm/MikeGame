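; BP_Button is an interactable button that triggers a list of affected actors when used and can be locked.
; Interact calls a server RPC, which checks Locked and sends either the use or locked sound to a client FX RPC played at the button's location.
; When unlocked, a client RPC also sends InteractMessage to each affected actor implementing BPI_Interaction.
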(event Custom|RPCClient_ButtonUse
  (for _array_element (Variables|Default|GetAffected%20Actors)
    (if (Utilities|DoesObjectImplementInterface _array_element "/Game/FirstPerson/Blueprints/BPI_Interaction.BPI_Interaction_C")
      (Class|BPIInteraction|Interact(Message) _array_element))))

(event Custom|RPCServer_ButtonUse
  (if (not (Variables|Default|GetLocked?))
    (CallFunction|RPCClientFX (Variables|Default|GetUseSound))
    (CallFunction|RPCClientButtonUse)
    (else
      (CallFunction|RPCClientFX (Variables|Default|GetLockedSound)))))

(event Custom|RPCClient_FX
  (params (Sound :type Sound%20Wave%20Object%20Reference))
  (Audio|PlaySoundatLocation Sound (Transformation|GetActorLocation) "0, 0, 0" 0.5 1.0 0.0 0 0 0 0))

(event EventInteract
  (CallFunction|RPCServerButtonUse))

(fn ConstructionScript)